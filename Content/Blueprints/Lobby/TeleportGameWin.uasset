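; TeleportGameWin is a teleport Blueprint in the Lobby folder that lets the player complete the stage.
; On BeginPlay it sets its DirectTxtWidget prompt to show the E key with "to complete stage".
; Its OnEnterLevel event opens the BattleVictoryWidget through the BattleGameModeBP UI manager instead of doing any travel itself.
; The parent class presumably supplies the interaction that fires OnEnterLevel, as none is defined here.
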(event EventBeginPlay
  (bind _asdirect_txt_widget (Utilities|Casting|CastToDirectTxtWidget (UserInterface|GetUserWidgetObject (Variables|Default|GetDirectTxtWidgetComponent))))
  (Default|SetInfo _asdirect_txt_widget "E" "to complete stage"))

(event Collision|EventActorBeginOverlap
  (params (OtherActor :type Actor%20Object%20Reference))
  (|CallParentFunction OtherActor) ; This node is disabled and will not be called.\nDrag off pins to build functionality.
)

(event EventTick
  (params (DeltaSeconds :type Float%20%28single-precision%29))
  (|CallParentFunction DeltaSeconds) ; This node is disabled and will not be called.\nDrag off pins to build functionality.
)

(event EventOnEnterLevel
  (bind _asbattle_game_mode_bp (Utilities|Casting|CastToBattleGameModeBP (Game|GetGameMode)))
  (Class|UIBaseMgr|OpenUI (Variables|/Script/Game3DtopdownRPG.BaseGameMode|GetUIMgr _asbattle_game_mode_bp) "BattleVictoryWidget" false false))

(fn ConstructionScript
  (|CallParentFunction))