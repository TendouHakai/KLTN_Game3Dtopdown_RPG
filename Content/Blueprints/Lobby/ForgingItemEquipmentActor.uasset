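; Lobby interaction actor for the item-forging station, which opens the forging screen when entered.
; On BeginPlay it sets its prompt widget to show the E key with a hint to open item forging.
; Its OnEnterLevel event opens the InternalPage scene through the battle game mode's UI manager and sets ForgingItem as that page's current building.
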(event EventBeginPlay
  (bind _asdirect_txt_widget (Utilities|Casting|CastToDirectTxtWidget (UserInterface|GetUserWidgetObject (Variables|Default|GetDirectTxtWidgetComponent))))
  (Default|SetInfo _asdirect_txt_widget "E" "to open forging Item"))

(event EventOnEnterLevel
  (bind _asbattle_game_mode_bp (Utilities|Casting|CastToBattleGameModeBP (Game|GetGameMode)))
  (bind _returnvalue (Class|UIBaseMgr|OpenScene (Variables|/Script/Game3DtopdownRPG.BaseGameMode|GetUIMgr _asbattle_game_mode_bp) "InternalPage"))
  (bind _asinternal_page (Utilities|Casting|CastToInternalPage _returnvalue))
  (Class|InternalWidget|SetCurrentBuilding _asinternal_page "ForgingItem"))

(fn ConstructionScript
  (|CallParentFunction))