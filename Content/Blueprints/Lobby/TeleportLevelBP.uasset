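; Lobby teleport actor that shows an "E to enter level" prompt when the player is in range.
; BeginPlay sets the text on its DirectTxtWidget component.
; Actor overlaps pass through OnPlayerInRange, which filters for PlayerCharacterBP with a BattleController and toggles the range flag and prompt.
; It binds an event to the controller's AdditionProc delegate on entry and unbinds all events from that delegate on exit.
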(event EventBeginPlay
  (bind _asdirect_txt_widget (Utilities|Casting|CastToDirectTxtWidget (UserInterface|GetUserWidgetObject (Variables|Default|GetDirectTxtWidgetComponent))))
  (Default|SetInfo _asdirect_txt_widget "E" "to enter level"))

(event EventTick
  (params (DeltaSeconds :type Float%20%28single-precision%29)))

(event Collision|EventActorBeginOverlap
  (params (OtherActor :type Actor%20Object%20Reference))
  (CallFunction|OnPlayerinRange true OtherActor))

(event Collision|EventActorEndOverlap
  (params (OtherActor :type Actor%20Object%20Reference))
  (CallFunction|OnPlayerinRange false OtherActor))

(fn ConstructionScript)

(fn OnPlayerinRange
  (params (IsInRange :type Boolean) (ACtor :type Actor%20Object%20Reference))
  (bind _asplayer_character_bp (Utilities|Casting|CastToPlayerCharacterBP ACtor))
  (bind _asbattle_controller (Utilities|Casting|CastToBattleController (Pawn|GetController _asplayer_character_bp)))
  (if IsInRange
    (EventDispatchers|BindEventtoAdditionProcDelegate _asbattle_controller (EventDispatchers|CreateEvent :!event OnEnterLevel))
    (else
      (EventDispatchers|UnbindallEventsfromAdditionProcDelegate _asbattle_controller)))
  (Class|TeleportLevel|SetIsPlayerinRange IsInRange)
  (bind _asdirect_txt_widget (Utilities|Casting|CastToDirectTxtWidget (UserInterface|GetUserWidgetObject (Variables|Default|GetDirectTxtWidgetComponent))))
  (Default|SetVisible _asdirect_txt_widget IsInRange))