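; Modular knight player character for battle that shows equipped items by swapping meshes per body slot.
; Body-part meshes follow the main Mesh through leader pose.
; After parent equip and unequip checks pass, a slot switch sets or resets meshes, with headgear also swapping to half hair.
; Hero class picks the hand for weapon and off-hand items; weapon changes update the character class, and equipping calls HeroMgr to unequip by class.
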(event Collision|EventActorBeginOverlap
  (params (OtherActor :type Actor%20Object%20Reference)))

(event EventBeginPlay
  (|CallParentFunction)
  (Components|SkinnedMesh|SetLeaderPoseComponent (Variables|Default|GetHair) (Variables|Character|GetMesh) false false))

(fn ConstructionScript)

(fn EquipItemtoPosition
  (params (Item%20reckey :type Integer) (ItemEquipmentInfoRecord :type Item%20Equipment%20Info%20Record%20Structure) (is%20Init :type Boolean))
  (bind _equipposition (Utilities|Struct|BreakItemEquipmentInfoRecord ItemEquipmentInfoRecord))
  (bind _is_valid (|CallParentFunction Item%20reckey ItemEquipmentInfoRecord is%20Init))
  (if _is_valid
    (LocalVariables|SetReckey Item%20reckey)
    (LocalVariables|SetPosition _equipposition)
    (switch Utilities|FlowControl|Switch|SwitchonEItemEquipPosition _equipposition
      (:HeadGears
        (Equipment|EquipHeadGear ItemEquipmentInfoRecord))
      (:ShoulderPad
        (Equipment|EquipShoulderPad ItemEquipmentInfoRecord))
      (:Shoe
        (Equipment|EquipShoe ItemEquipmentInfoRecord))
      (:Glove
        (Equipment|EquipGlove ItemEquipmentInfoRecord))
      (:Belt
        (Equipment|EquipBelt ItemEquipmentInfoRecord))
      (:Backpack
        (Equipment|EquipBackpack ItemEquipmentInfoRecord))
      (:Weapon
        (Equipment|EquipWeapon ItemEquipmentInfoRecord))
      (:Shield
        (Equipment|EquipShield ItemEquipmentInfoRecord))
      (:Clother
        (Equipment|EquipClother ItemEquipmentInfoRecord)))
    (return true)
    (else
      (return false))))

(fn EquipHeadGear
  (params (Item%20Info :type Item%20Equipment%20Info%20Record%20Structure))
  (Components|SkeletalMesh|SetSkeletalMeshAsset (Variables|Default|GetHeadGears) (.MeshSkeletal (Utilities|Struct|BreakItemEquipmentInfoRecord Item%20Info)))
  (Components|SkeletalMesh|SetSkeletalMeshAsset (Variables|Default|GetHair) "/Game/ModularRPGHeroesPBR/Meshes/ModularBodyParts/Hair01HalfSK.Hair01HalfSK"))

(fn EquipShoulderPad
  (params (ItemInfo :type Item%20Equipment%20Info%20Record%20Structure))
  (Components|SkeletalMesh|SetSkeletalMeshAsset (Variables|Default|GetShoulderPad) (.MeshSkeletal (Utilities|Struct|BreakItemEquipmentInfoRecord ItemInfo))))

(fn EquipShoe
  (params (Item%20Info :type Item%20Equipment%20Info%20Record%20Structure))
  (Components|SkeletalMesh|SetSkeletalMeshAsset (Variables|Default|GetShoe) (.MeshSkeletal (Utilities|Struct|BreakItemEquipmentInfoRecord Item%20Info))))

(fn EquipGlove
  (params (Item%20Info :type Item%20Equipment%20Info%20Record%20Structure))
  (Components|SkeletalMesh|SetSkeletalMeshAsset (Variables|Default|GetGlove) (.MeshSkeletal (Utilities|Struct|BreakItemEquipmentInfoRecord Item%20Info))))

(fn EquipBelt
  (params (Item%20Info :type Item%20Equipment%20Info%20Record%20Structure))
  (Components|SkeletalMesh|SetSkeletalMeshAsset (Variables|Default|GetBelt) (.MeshSkeletal (Utilities|Struct|BreakItemEquipmentInfoRecord Item%20Info))))

(fn EquipWeapon
  (params (ItemInfo :type Item%20Equipment%20Info%20Record%20Structure))
  (bind (_desname _equipmentlevel _equipmentgrape _equipposition _itemequipparam _previousitem _needgold _sellgold _materials _matcounts _meshskeletal _meshstatic _iconname _itemparamlevid _heroclass) (Utilities|Struct|BreakItemEquipmentInfoRecord ItemInfo))
  (switch Utilities|FlowControl|Switch|SwitchonEHeroClass _heroclass
    (:SwordAndShield
      (Components|StaticMesh|SetStaticMesh (Variables|Default|GetRightWeapon) _meshstatic :!label _label))
    (:Bow
      (Components|StaticMesh|SetStaticMesh (Variables|Default|GetLeftWeapon) _meshstatic :!label _label_2))
    (:DoubleSword
      (goto _label))
    (:MagicWand
      (goto _label))
    (:SingleSword
      (goto _label_2)))
  (Variables|Default|SetcurrentCharacterClass _heroclass)
  (Class|HeroMgr|UnEquipHeroItembyClass (Class|CppFunctionLibrary|GetHeroMgr) self))

(fn EquipShield
  (params (Item%20Info :type Item%20Equipment%20Info%20Record%20Structure))
  (bind (_desname _equipmentlevel _equipmentgrape _equipposition _itemequipparam _previousitem _needgold _sellgold _materials _matcounts _meshskeletal _meshstatic _iconname _itemparamlevid _heroclass) (Utilities|Struct|BreakItemEquipmentInfoRecord Item%20Info))
  (switch Utilities|FlowControl|Switch|SwitchonEHeroClass _heroclass
    (:SwordAndShield
      (Components|StaticMesh|SetStaticMesh (Variables|Default|GetShield) _meshstatic))
    (:Bow
      (Components|StaticMesh|SetStaticMesh (Variables|Default|GetRightWeapon) _meshstatic))
    (:DoubleSword
      (Components|StaticMesh|SetStaticMesh (Variables|Default|GetLeftWeapon) _meshstatic))))

(fn EquipBackpack
  (params (Item%20Info :type Item%20Equipment%20Info%20Record%20Structure))
  (Components|StaticMesh|SetStaticMesh (Variables|Default|GetBackpack) (.MeshStatic (Utilities|Struct|BreakItemEquipmentInfoRecord Item%20Info))))

(fn EquipClother
  (params (Item%20Info :type Item%20Equipment%20Info%20Record%20Structure))
  (Components|SkeletalMesh|SetSkeletalMeshAsset (Variables|Character|GetMesh) (.MeshSkeletal (Utilities|Struct|BreakItemEquipmentInfoRecord Item%20Info))))

(fn UnEquipmenttoPosition
  (params (ItemReckey :type Integer) (ItemEquipment%20Info%20Record :type Item%20Equipment%20Info%20Record%20Structure))
  (bind _isvalid (|CallParentFunction ItemReckey ItemEquipment%20Info%20Record))
  (if _isvalid
    (switch Utilities|FlowControl|Switch|SwitchonEItemEquipPosition (.EquipPosition (Utilities|Struct|BreakItemEquipmentInfoRecord ItemEquipment%20Info%20Record))
      (:HeadGears
        (Equipment|UnEquipHeadGear ItemEquipment%20Info%20Record))
      (:ShoulderPad
        (Equipment|UnEquipShoulderPad ItemEquipment%20Info%20Record))
      (:Shoe
        (Equipment|UnEquipShoe ItemEquipment%20Info%20Record))
      (:Glove
        (Equipment|UnEquipGlove ItemEquipment%20Info%20Record))
      (:Belt
        (Equipment|UnEquipBelt ItemEquipment%20Info%20Record))
      (:Backpack
        (Equipment|UnEquipBackpack ItemEquipment%20Info%20Record))
      (:Weapon
        (Equipment|UnEquipWeapon ItemEquipment%20Info%20Record))
      (:Shield
        (Equipment|UnEquipShield ItemEquipment%20Info%20Record))
      (:Clother
        (Equipment|UnEquipClother ItemEquipment%20Info%20Record)))
    (return true)
    (else
      (return false))))

(fn UnEquipHeadGear
  (params (Item%20Info :type Item%20Equipment%20Info%20Record%20Structure))
  (Components|SkeletalMesh|SetSkeletalMeshAsset (Variables|Default|GetHeadGears) 0)
  (Components|SkeletalMesh|SetSkeletalMeshAsset (Variables|Default|GetHair) "/Game/ModularRPGHeroesPBR/Meshes/ModularBodyParts/Hair01SK.Hair01SK"))

(fn UnEquipShoulderPad
  (params (Item%20Info :type Item%20Equipment%20Info%20Record%20Structure))
  (Components|SkeletalMesh|SetSkeletalMeshAsset (Variables|Default|GetShoulderPad) 0))

(fn UnEquipShoe
  (params (Item%20Info :type Item%20Equipment%20Info%20Record%20Structure))
  (Components|SkeletalMesh|SetSkeletalMeshAsset (Variables|Default|GetShoe) "/Game/ModularRPGHeroesPBR/Meshes/ModularBodyParts/Shoe01SK.Shoe01SK"))

(fn UnEquipGlove
  (params (Item%20Info :type Item%20Equipment%20Info%20Record%20Structure))
  (Components|SkeletalMesh|SetSkeletalMeshAsset (Variables|Default|GetGlove) "/Game/ModularRPGHeroesPBR/Meshes/ModularBodyParts/Glove01SK.Glove01SK"))

(fn UnEquipBelt
  (params (Item%20Info :type Item%20Equipment%20Info%20Record%20Structure))
  (Components|SkeletalMesh|SetSkeletalMeshAsset (Variables|Default|GetBelt) "/Game/ModularRPGHeroesPBR/Meshes/ModularBodyParts/Glove01SK.Glove01SK"))

(fn UnEquipWeapon
  (params (Item%20Info :type Item%20Equipment%20Info%20Record%20Structure))
  (switch Utilities|FlowControl|Switch|SwitchonEHeroClass (.HeroClass (Utilities|Struct|BreakItemEquipmentInfoRecord Item%20Info))
    (:NoWeapon
      (Components|StaticMesh|SetStaticMesh (Variables|Default|GetRightWeapon) 0 :!label _label))
    (:SwordAndShield
      (goto _label))
    (:Bow
      (Components|StaticMesh|SetStaticMesh (Variables|Default|GetLeftWeapon) 0 :!label _label_2))
    (:DoubleSword
      (goto _label))
    (:MagicWand
      (goto _label))
    (:SingleSword
      (goto _label_2)))
  (Variables|Default|SetcurrentCharacterClass "NoWeapon"))

(fn UnEquipShield
  (params (Item%20Info :type Item%20Equipment%20Info%20Record%20Structure))
  (switch Utilities|FlowControl|Switch|SwitchonEHeroClass (.HeroClass (Utilities|Struct|BreakItemEquipmentInfoRecord Item%20Info))
    (:SwordAndShield
      (Components|StaticMesh|SetStaticMesh (Variables|Default|GetShield) 0))
    (:Bow
      (Components|StaticMesh|SetStaticMesh (Variables|Default|GetRightWeapon) 0))
    (:DoubleSword
      (Components|StaticMesh|SetStaticMesh (Variables|Default|GetLeftWeapon) 0))))

(fn UnEquipBackpack
  (params (Item%20Info :type Item%20Equipment%20Info%20Record%20Structure))
  (Components|StaticMesh|SetStaticMesh (Variables|Default|GetBackpack) 0))

(fn UnEquipClother
  (params (Item%20Info :type Item%20Equipment%20Info%20Record%20Structure))
  (Components|SkeletalMesh|SetSkeletalMeshAsset (Variables|Character|GetMesh) "/Game/ModularRPGHeroesPBR/Meshes/ModularBodyParts/Cloth01SK.Cloth01SK"))