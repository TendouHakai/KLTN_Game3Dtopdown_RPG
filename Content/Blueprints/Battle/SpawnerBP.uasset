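; Battle spawner actor that spawns a configured character class on a given team and optionally destroys itself afterwards.
; In editor it previews that class's skeletal mesh, hidden at BeginPlay.
; Spawn transforms cancel the character's relative mesh offset and rotation, aligning the spawned mesh with the spawner.
; Boss spawns set the AI controller's cooldown and notify BattleGameModeBP; otherwise, spawned gimmicks receive repeat and start-time settings.
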(event EventBeginPlay
  (Rendering|SetVisibility (Variables|Default|GetSkeletalMeshComponent) false false))

(fn ConstructionScript
  (if (Class|Utility|IsEditorPlay)
    (bind _returnvalue (Class|CppFunctionLibrary|GetDefaultObject (Variables|Spawner|GetCharacterClass)))
    (bind _asbase_character_bp (Utilities|Casting|CastToBaseCharacterBP _returnvalue))
    (Components|SkeletalMesh|SetSkeletalMeshAsset (Variables|Default|GetSkeletalMeshComponent) (Variables|/Script/Engine.SkeletalMeshComponent|GetSkeletalMeshAsset (Variables|/Script/Engine.Character|GetMesh _asbase_character_bp)))))

(fn SpawnActor
  (LocalVariables|SetSpawnCharacterClass (Variables|Spawner|GetCharacterClass))
  (if (Utilities|IsValidClass (LocalVariables|GetSpawnCharacterClass))
    (bind _tranform (CallFunction|CalcSpawnTransform (LocalVariables|GetSpawnCharacterClass)))
    (bind _returnvalue (Game|SpawnActorfromClass (LocalVariables|GetSpawnCharacterClass) _tranform "AlwaysSpawn" "MultiplyWithRoot" 0 "Enemy" (Variables|Spawner|GetLevel) 0))
    (Variables|Spawner|SetSpawnerActor _returnvalue)
    (Class|BaseCharacter|SetCharTeam _returnvalue (Variables|Spawner|GetCharTeam))
    (if (Variables|Spawner|GetbBoss)
      (bind _asaiboss_controller (Utilities|Casting|CastToAIBossController (Pawn|GetController _returnvalue)))
      (Default|SetWorldBossCoolTime _asaiboss_controller)
      (bind _asbattle_game_mode_bp (Utilities|Casting|CastToBattleGameModeBP (Game|GetGameMode)))
      (Default|OnBossSpawn _asbattle_game_mode_bp _returnvalue)
      (else
        (bind _asbase_gimmick_repeatition (Utilities|Casting|CastToBaseGimmickRepeatition _returnvalue)
          (:then
            (Variables|/Game/Blueprints/Battle/EnemyCharacter/Gimmick/BaseGimmickRepeatition.BaseGimmickRepeatition_C|SetbRepeatition _asbase_gimmick_repeatition (Variables|Gimmick|GetGimmickIsRepeat))
            (Variables|/Game/Blueprints/Battle/EnemyCharacter/Gimmick/BaseGimmickRepeatition.BaseGimmickRepeatition_C|SetNumberToRepeatition _asbase_gimmick_repeatition (Variables|Gimmick|GetGimmickNumberRepeat))
            (Default|SetStartTime _asbase_gimmick_repeatition (Variables|Gimmick|GetGimmickStartTime)))
          (:CastFailed
            _))))
    (if (Variables|Spawner|GetbOnceSpawn)
      (Actor|DestroyActor)))
  (return (Variables|Spawner|GetSpawnerActor)))

(fn CalcSpawnTransform
  (params (Object%20Class :type Object%20Class%20Reference))
  (bind _returnvalue (Class|CppFunctionLibrary|GetDefaultObject Object%20Class))
  (bind _asactor (Utilities|Casting|CastToActor _returnvalue)
    (:then
      (bind (_returnlocation _returnrotation) (CallFunction|CalcLocation&Rotation _asactor)))
    (:CastFailed
      _))
  (return (Math|Transform|MakeTransform _returnlocation _returnrotation (Transformation|GetActorScale3D))))

(fn CalcLocation&Rotation
  (params (SpawnerActor :type Actor%20Object%20Reference))
  (LocalVariables|SetreturnLoc (Transformation|GetActorLocation))
  (LocalVariables|SetreturnRot (Transformation|GetActorRotation))
  (bind _ascharacter (Utilities|Casting|CastToCharacter SpawnerActor)
    (:then
      (Utilities|FlowControl|Sequence
        (:then_0
          (LocalVariables|SetreturnRot (Math|Rotator|CombineRotators (LocalVariables|GetreturnRot) (Class|KismetMathLibrary|NegateRotator (Variables|/Script/Engine.SceneComponent|GetRelativeRotation (Variables|/Script/Engine.Character|GetMesh _ascharacter))))))
        (:then_1
          (LocalVariables|SetreturnLoc (+ (LocalVariables|GetreturnLoc) (Math|Vector|RotateVector (Math|Vector|NegateVector (Variables|/Script/Engine.SceneComponent|GetRelativeLocation (Variables|/Script/Engine.Character|GetMesh _ascharacter))) (LocalVariables|GetreturnRot))))
          (return (LocalVariables|GetreturnLoc) (LocalVariables|GetreturnRot)))))
    (:CastFailed
      (return (LocalVariables|GetreturnLoc) (LocalVariables|GetreturnRot)))))

(fn GetCharacterClass
  (return (Variables|Spawner|GetCharacterClass)))

(fn Spawn
  (bind _spawneractor (CallFunction|SpawnActor))
  (return _spawneractor))