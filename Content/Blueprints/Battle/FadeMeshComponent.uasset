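; FadeMeshComponent is a battle component that swaps its owner's static mesh materials to a fade material and back.
; BeginPlay caches the owner's first StaticMeshComponent.
; OnFade saves the current materials in OriginMat, then applies FadeMaterial to every slot, while ExitFade restores the saved materials by index.
; The swap is instant, with no blending or timing in the component itself.
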(event EventBeginPlay
  (Variables|Default|SetStaticMeshComponent (Actor|GetComponentbyClass (Components|GetOwner) "/Script/Engine.StaticMeshComponent")))

(fn OnFade
  (bind _staticmeshcomponent (Variables|Default|GetStaticMeshComponent))
  (bind _returnvalue (Rendering|Material|GetMaterials _staticmeshcomponent))
  (Utilities|Array|Clear (Variables|Default|GetOriginMat))
  (Utilities|IsValid _staticmeshcomponent
    (:Is%20Valid
      (for _array_element _returnvalue
        (Utilities|Array|Add (Variables|Default|GetOriginMat) _array_element))
      (for _index (range 0 (- (Utilities|Array|Length _returnvalue) 1))
        (Rendering|Material|SetMaterial (Variables|Default|GetStaticMeshComponent) _index "/Game/Legendary_Forge/Materials/FadeMaterial.FadeMaterial")))))

(fn ExitFade
  (Utilities|IsValid (Variables|Default|GetStaticMeshComponent)
    (:Is%20Valid
      (for _index (range 0 (- (Utilities|Array|Length (Variables|Default|GetOriginMat)) 1))
        (Rendering|Material|SetMaterial (Variables|Default|GetStaticMeshComponent) _index (Utilities|Array|Get(acopy) (Variables|Default|GetOriginMat) _index))))))