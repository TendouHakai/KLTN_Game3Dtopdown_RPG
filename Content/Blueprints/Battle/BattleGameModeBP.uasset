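; Battle game mode that sets up the battle UI, player and boss encounter flow.
; On login it caches the BattlePlayerController, spawns and possesses the hero at a player start, then applies hero buff info when production begins.
; Boss directing hides the spawner during the cinematic, then hides matinee actors and spawns the boss.
; Boss spawn and death toggle the health bar, while BattleClearComponentBP handles failure and the win teleport.
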(event EventPostLogin
  (params (NewPlayer :type Player%20Controller%20Object%20Reference))
  (|CallParentFunction NewPlayer)
  (|InitBattleController NewPlayer)
  (|InitPlayerCharacter))

(event EventOnBeginProduction
  (CallFunction|SetBuffInfoHero))

(event EventOnInitInitialUI
  (Class|UIBaseMgr|OpenScene (Variables|Default|GetUIMgr) "BattleWidget")
  (Default|InitUI (Variables|Components|GetBattleController)))

(fn ConstructionScript)

(fn PlayerCharacterDied
  (Class|BattleClearComponent|SetBattleClearStep (Variables|Default|GetBattleClearComponentBP) "Failed"))

(fn OnBossSpawn
  (params (Boss :type Base%20Character%20BP%20Object%20Reference))
  (LocalVariables|SetBossActor Boss)
  (bind _returnvalue (Class|UIBaseMgr|OpenUI (Variables|Default|GetUIMgr) "BattleBossProgessWidget" false false))
  (Variables|Boss|SetBossWidget _returnvalue)
  (bind _asboss_health_bar (Utilities|Casting|CastToBossHealthBar (Variables|Boss|GetBossWidget)))
  (Variables|/Game/UI/Widgets/Battle/BossHealthBar.BossHealthBar_C|SetOwnerCharacter _asboss_health_bar (LocalVariables|GetBossActor)))

(fn BossDied
  (Class|UIBaseMgr|CloseUI (Variables|Default|GetUIMgr) "BattleBossProgessWidget" false true)
  (Class|BattleClearComponent|ShowTeleportWin (Variables|Default|GetBattleClearComponentBP)))

(fn BeginBossDirecting
  (params (SpawnerBoss :type Spawner%20BP%20Object%20Reference) (ActorsInMatinee :type Array%20of%20Actor%20Object%20References))
  (bind _output_get (Variables|Boss|SetBossSpawner SpawnerBoss))
  (Rendering|SetActorHiddenInGame _output_get true)
  (Variables|Boss|SetActorsInMatinee ActorsInMatinee))

(fn EndBossDirecting
  (|HideActorInMatinee
    (:LoopBody
      (|ShowAllCharacters)
      (Default|SpawnActor (Variables|Boss|GetBossSpawner)))))

(fn SetTeleportWin
  (params (Teleport :type Teleport%20Game%20Win%20Object%20Reference))
  (Class|BattleClearComponent|SetTeleportWin (Variables|Default|GetBattleClearComponentBP) Teleport))

(fn SetBuffInfoHero
  (Default|SetHeroBuffInfo (Variables|Components|GetBattleController) (Variables|Default|GetCharacter)))

(fn InitPlayerCharacter
  (params (PlayerTranform :type Transform))
  (bind _character (Variables|Default|GetCharacter))
  (Utilities|FlowControl|Sequence
    (:then_0
      (CallFunction|AddPlayerCharacter (Variables|Default|GetPlayerCharacterClass) PlayerTranform true))
    (:then_1
      (Pawn|Possess (Variables|Components|GetBattleController) _character)
      (Default|SetVisible _character true))))

(fn AddPlayerCharacter
  (params (PlayerClass :type Player%20Character%20BP%20Class%20Reference) (PlayerTranform :type Transform) (Visible :type Boolean))
  (bind _returnvalue (Game|SpawnActorfromClass PlayerClass PlayerTranform "Undefined" "MultiplyWithRoot" 0 "Ally" 0))
  (bind _output_get (Variables|Default|SetCharacter _returnvalue))
  (Default|SetVisible _output_get Visible))