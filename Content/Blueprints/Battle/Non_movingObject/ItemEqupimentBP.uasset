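; Equipment item drop for battle, built on a coin-style pickup parent, that goes into the player's backpack when picked.
; A widget component displays the item's info, filled on BeginPlay and again whenever SetGameInfo supplies new data.
; On pickup, it reads the record key and upgrade level back from that widget, adds the equipment through the item manager and destroys itself.
; A coin sound plays when the chase starts.
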(event Custom|Picked
  (params (PickedCoin :type Coin%20Object%20Reference))
  (bind _asinventory_equipment_container_widget (Utilities|Casting|CastToInventoryEquipmentContainerWidget (UserInterface|GetWidget (Variables|Default|GetWidget))))
  (Class|ItemMgr|AddItemEquipment (Class|CppFunctionLibrary|GetItemMgr) (.m_ItemRecKey (Utilities|Struct|BreakGameItemEquipmentInfo (Class|InventoryEquipContainerWidget|GetGameItemInfo _asinventory_equipment_container_widget))) (.m_ItemUgrapeLevel (Utilities|Struct|BreakGameItemEquipmentInfo (Class|InventoryEquipContainerWidget|GetGameItemInfo _asinventory_equipment_container_widget))) "InBackpack")
  (Actor|DestroyActor))

(event EventOnCoinStartChase
  (Audio|SpawnSoundatLocation "/Game/Sound/Coin_Sfx_01_Cue.Coin_Sfx_01_Cue" (Transformation|GetActorLocation) "0, 0, 0" 1.0 1.0 0.0 0 0))

(event EventBeginPlay
  (|CallParentFunction)
  (bind _asinventory_equipment_container_widget (Utilities|Casting|CastToInventoryEquipmentContainerWidget (UserInterface|GetWidget (Variables|Default|GetWidget))))
  (Class|InventoryEquipContainerWidget|CacheOwnUI _asinventory_equipment_container_widget)
  (Class|InventoryEquipContainerWidget|SetInfo _asinventory_equipment_container_widget (Variables|Default|GetGameItemEquipInfo))
  (EventDispatchers|BindEventtoOnCoinPicked (delegate Custom|Picked)))

(event EventTick
  (params (DeltaSeconds :type Float%20%28single-precision%29))
  (|CallParentFunction DeltaSeconds))

(fn ConstructionScript)

(fn SetGameInfo
  (params (GameItemInfo :type Game%20Item%20Equipment%20Info%20Structure))
  (Variables|Default|SetGameItemEquipInfo GameItemInfo)
  (bind _asinventory_equipment_container_widget (Utilities|Casting|CastToInventoryEquipmentContainerWidget (UserInterface|GetWidget (Variables|Default|GetWidget))))
  (Class|InventoryEquipContainerWidget|CacheOwnUI _asinventory_equipment_container_widget)
  (Class|InventoryEquipContainerWidget|SetInfo _asinventory_equipment_container_widget (Variables|Default|GetGameItemEquipInfo)))