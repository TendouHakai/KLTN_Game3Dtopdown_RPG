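; Battle pickup actor for a dropped game item, built on a coin-pickup parent that provides the chase and picked events.
; An inventory container widget displays the item's info, filled at BeginPlay and again through SetGameInfo.
; When picked, it reads the item key and count back from the widget, adds them to the backpack via the item manager and destroys itself.
; A coin sound plays at its location when the chase starts.
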(event Custom|Picked
  (params (PickedCoin :type Coin%20Object%20Reference))
  (bind _asmy_inventory_container_widget (Utilities|Casting|CastToMyInventoryContainerWidget (UserInterface|GetWidget (Variables|Default|GetWidget))))
  (Class|ItemMgr|AddItem (Class|CppFunctionLibrary|GetItemMgr) (.m_ItemRecKey (Utilities|Struct|BreakGameItemInfo (Class|InventoryContainerWidget|GetGameItemInfo _asmy_inventory_container_widget))) (.m_ItemCount (Utilities|Struct|BreakGameItemInfo (Class|InventoryContainerWidget|GetGameItemInfo _asmy_inventory_container_widget))) "InBackpack")
  (Actor|DestroyActor))

(event EventOnCoinStartChase
  (Audio|SpawnSoundatLocation "/Game/Sound/Coin_Sfx_01_Cue.Coin_Sfx_01_Cue" (Transformation|GetActorLocation) "0, 0, 0" 1.0 1.0 0.0 0 0))

(event EventBeginPlay
  (|CallParentFunction)
  (bind _asmy_inventory_container_widget (Utilities|Casting|CastToMyInventoryContainerWidget (UserInterface|GetWidget (Variables|Default|GetWidget))))
  (Class|InventoryContainerWidget|CacheOwnUI _asmy_inventory_container_widget)
  (Class|InventoryContainerWidget|SetInfo _asmy_inventory_container_widget (Variables|Default|GetGameItemInfo))
  (EventDispatchers|BindEventtoOnCoinPicked (delegate Custom|Picked)))

(event EventTick
  (params (DeltaSeconds :type Float%20%28single-precision%29))
  (|CallParentFunction DeltaSeconds))

(fn ConstructionScript)

(fn SetGameInfo
  (params (GameItemInfo :type Game%20Item%20Info%20Structure))
  (Variables|Default|SetGameItemInfo GameItemInfo)
  (bind _asmy_inventory_container_widget (Utilities|Casting|CastToMyInventoryContainerWidget (UserInterface|GetWidget (Variables|Default|GetWidget))))
  (Class|InventoryContainerWidget|CacheOwnUI _asmy_inventory_container_widget)
  (Class|InventoryContainerWidget|SetInfo _asmy_inventory_container_widget (Variables|Default|GetGameItemInfo)))