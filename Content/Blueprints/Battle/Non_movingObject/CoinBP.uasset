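; CoinBP is a battle gold coin pickup that awards gold to the player when picked.
; On BeginPlay it creates a gold text widget and binds the parent's coin-picked event, whose handler shows the amount at the coin's location, adds it through the item manager and destroys the actor.
; It plays a coin sound when the chase starts.
; DestroyCoin removes the widget and destroys the coin.
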(event Custom|ShowGoldTxt
  (params (PickedCoin :type Coin%20Object%20Reference))
  (bind _goldtxtwidget (Variables|Default|GetGoldTxtWidget))
  (Default|InitGoldTxt _goldtxtwidget (Transformation|GetActorLocation) (Variables|Default|GetGoldAmount))
  (UserInterface|Viewport|AddtoViewport _goldtxtwidget 0)
  (Class|ItemMgr|AddGold (Class|CppFunctionLibrary|GetItemMgr) (Class|KismetMathLibrary|ToInt64(Integer) (Variables|Default|GetGoldAmount)))
  (Actor|DestroyActor))

(event EventOnCoinStartChase
  (Audio|SpawnSoundatLocation "/Game/Sound/Coin_Sfx_01_Cue.Coin_Sfx_01_Cue" (Transformation|GetActorLocation) "0, 0, 0" 1.0 1.0 0.0 0 0))

(event EventBeginPlay
  (|CallParentFunction)
  (bind _returnvalue (UserInterface|CreateWidget "/Game/UI/Widgets/Battle/CoinTxtWidget.CoinTxtWidget_C" (Game|GetPlayerController 0)))
  (Variables|Default|SetGoldTxtWidget _returnvalue)
  (EventDispatchers|BindEventtoOnCoinPicked (delegate Custom|ShowGoldTxt)))

(event EventTick
  (params (DeltaSeconds :type Float%20%28single-precision%29))
  (|CallParentFunction DeltaSeconds))

(fn ConstructionScript)

(fn DestroyCoin
  (Widget|RemovefromParent (Variables|Default|GetGoldTxtWidget))
  (Actor|DestroyActor))