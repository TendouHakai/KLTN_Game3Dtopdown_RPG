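; Damage component for BaseCharacterBP owners that handles both dealing and receiving hits in battle.
; Outgoing attacks spawn a projectile or briefly enable a sphere's collision to damage overlapping enemies and apply buffs, crediting trap casters for buffs.
; Incoming damage checks invincibility and dodging through dashing or attacker blindness, then applies hit freeze, health change, damage text and hit or death handling.
; Damage-over-time skips damage calculation, knockback and hit animation.
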(event EventBeginPlay
  (bind _asbase_character_bp (Utilities|Casting|CastToBaseCharacterBP (Components|GetOwner)))
  (Variables|Default|SetOwnerCharacter _asbase_character_bp))

(fn DamageEnemtin
  (params (SphereRadius :type Shape%20Component%20Object%20Reference) (DamageInfo :type Base%20Damage%20Info%20Structure) (HeroBuffInfo :type Hero%20Buff%20Info%20Structure))
  (bind _ownercharacter (Variables|Default|GetOwnerCharacter))
  (bind _attacker (CallFunction|GetAttackerCharacter _ownercharacter))
  (if (|IsProjectileAttack DamageInfo)
    (CallFunction|SpawnProjectile DamageInfo HeroBuffInfo)
    (else
      (Class|BaseCharacter|AddBufftoAttacker _attacker _attacker HeroBuffInfo)
      (Collision|SetCollisionEnabled SphereRadius "QueryAndPhysics")
      (bind (_outenemyteam _returnvalue) (Class|BaseCharacter|GetEnemyTeam (Variables|Default|GetOwnerCharacter)))
      (if _returnvalue
        (bind _actors (CallFunction|GetOverlapEnemy SphereRadius _outenemyteam))
        (for _array_element _actors
          (if (and (Class|BaseCharacter|IsCharacterDamageable _array_element) (!= _array_element (Variables|Default|GetOwnerCharacter)))
            (bind _hitsuccess (Default|CharacterDamaged _array_element DamageInfo (Variables|Default|GetOwnerCharacter) false))
            (if _hitsuccess
              (Class|BaseCharacter|AddBufftoDefender _array_element (CallFunction|GetAttackerCharacter (Variables|Default|GetOwnerCharacter)) HeroBuffInfo))))
        (Collision|SetCollisionEnabled SphereRadius "NoCollision")))))

(fn GetOverlapEnemy
  (params (SphereRadius :type Shape%20Component%20Object%20Reference) (EnemtTeam :type ECharTeam%20Enum :default "Ally"))
  (for _array_element (Collision|GetOverlappingActors SphereRadius "/Game/Blueprints/Battle/BaseCharacterBP.BaseCharacterBP_C" :!class /Script/Engine.PrimitiveComponent)
    (bind _asbase_character_bp (Utilities|Casting|CastToBaseCharacterBP _array_element))
    (bind _returnvalue (Class|BaseCharacter|GetCharTeam _asbase_character_bp))
    (if (Utilities|Enum|Equal(Enum) _returnvalue EnemtTeam)
      (Utilities|Array|Add (LocalVariables|GetActorTemps) _asbase_character_bp)))
  (return (LocalVariables|GetActorTemps)))

(fn CharacterDamaged
  (params (DamageInfo :type Base%20Damage%20Info%20Structure) (Attacker :type Base%20Character%20BP%20Object%20Reference) (Damage%20By%20Dot :type Boolean))
  (|Setlocalvariables DamageInfo Attacker Damage%20By%20Dot)
  (bind _returnvalue (Class|BaseCharacter|IsInvincible (Variables|Default|GetOwnerCharacter)))
  (if (not _returnvalue)
    (|ProcDodge (LocalVariables|GetAttackerCharacter)
      (:IsDodge
        (return false))
      (:NotIsDodge
        (if (Variables|Default|GetbDamageDot)
          _
          (else
            (Default|CalculateDamage (Variables|Default|GetOwnerCharacter) (LocalVariables|GetAttackerCharacter) (LocalVariables|GetBaseDamageInfo))
            (Default|KnockbackLocation (Variables|Default|GetOwnerCharacter) (LocalVariables|GetAttackerCharacter) (.KnockbackDistance (Utilities|Struct|BreakBaseDamageInfo (LocalVariables|GetBaseDamageInfo))))))
        (Utilities|FlowControl|Sequence
          (:then_0
            (|DamageProcess))
          (:then_1
            (|DamageInfo))
          (:then_2
            (if (> (Class|BaseCharacter|GetHP (Variables|Default|GetOwnerCharacter)) 0.0)
              (|HitProcess)
              (else
                (|DieProcess))))
          (:then_3
            (return true)))))))

(fn SpawnProjectile
  (params (DamageInfo :type Base%20Damage%20Info%20Structure) (HeroBuffInfo :type Hero%20Buff%20Info%20Structure))
  (bind _return_object (|Spawn DamageInfo))
  (bind _outenemyteam (Class|BaseCharacter|GetEnemyTeam (Variables|Default|GetOwnerCharacter)))
  (Default|InitProjectile _return_object _outenemyteam DamageInfo HeroBuffInfo (Variables|Default|GetOwnerCharacter)))

(fn GetAttackerCharacter
  (params (Character :type Base%20Character%20BP%20Object%20Reference))
  (bind _asplayer_trap (Utilities|Casting|CastToPlayerTrap Character)
    (:then
      (return (Variables|/Game/Blueprints/Battle/EnemyCharacter/PlayerSummon/PlayerSummon.PlayerSummon_C|GetCaster _asplayer_trap)))
    (:CastFailed
      (return Character))))