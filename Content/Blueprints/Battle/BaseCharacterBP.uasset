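; Base battle character Blueprint that links the character to its animation Blueprint.
; On BeginPlay it casts the mesh's anim instance to BaseAnimBP_Template and caches it.
; UpdateRunningSpeed writes scaled movement velocity magnitude into that anim Blueprint, though nothing in this graph calls it.
; IsMovable defers to the anim state, returning true during either attack or movable states.
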(event EventBeginPlay
  (Init|InitAnimBP))

(event Collision|EventActorBeginOverlap
  (params (OtherActor :type Actor%20Object%20Reference)))

(event EventTick
  (params (DeltaSeconds :type Float%20%28single-precision%29)))

(fn ConstructionScript)

(fn CalRunningSpeed
  (return (* (Math|Vector|VectorLength (Variables|/Script/Engine.MovementComponent|GetVelocity (Variables|Character|GetCharacterMovement))) 5e+01)))

(fn UpdateRunningSpeed
  (bind _runningspeed (CallFunction|CalRunningSpeed))
  (Variables|/Game/Blueprints/Battle/BaseAnimBP_Template.BaseAnimBP_Template_C|SetRunningSpeed (Variables|Default|GetanimBP) _runningspeed))

(fn InitAnimBP
  (bind _asbase_anim_bp_template (Utilities|Casting|CastToBaseAnimBP_Template (Components|SkeletalMesh|GetAnimInstance (Variables|Character|GetMesh))))
  (Variables|Default|SetanimBP _asbase_anim_bp_template))

(fn IsMovable
  (bind _animbp (Variables|Default|GetanimBP))
  (return (or (Class|BaseAnimInstance|IsAnimAttackState _animbp) (Class|BaseAnimInstance|IsAnimMovable _animbp))))