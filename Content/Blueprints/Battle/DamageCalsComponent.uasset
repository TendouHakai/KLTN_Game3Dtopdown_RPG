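; Battle component that holds an actor's attack, defense, piercing and critical stats and calculates damage received from an attacker.
; CalsDamage scales damage by the attacker component's physical or magic attack, CalcDef and a random 2x critical, then prints it.
; CalcDef contains an unwired 600/(defense minus pierce + 600) mitigation formula, with defense floored at zero.
; ApplyBaseParams loads stats, taking critical ratio from DebuffResistanceRatio; ParsingDamageCalcInfo copies offensive stats from another component.
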(fn CalsDamage
  (params (Attacker :type Base%20Character%20BP%20Object%20Reference) (DamageAmount :type Float%20%28double-precision%29%20%28by%20ref%29) (IsMagicDamage :type Boolean))
  (LocalVariables|SetisMagic IsMagicDamage)
  (bind _elem (Utilities|GetatSafe (Actor|GetComponentsByClass Attacker "DamageCalsComponent_C"))
    (:Success
      (bind _output_get (LocalVariables|SetAttackerDamageCalsComponent _elem))
      (bind (_sumcriticalratio _sumcriticaldamageratio) (CallFunction|CalcCriticalRatio _output_get))
      (LocalVariables|SetIsCritical (<= (Math|Random|RandomFloatinRange 0.0 1.0) _sumcriticalratio))
      (LocalVariables|SetSumCriticalDamageRatio _sumcriticaldamageratio)
      (|SetBy-RefVar DamageAmount (* DamageAmount (select (LocalVariables|GetisMagic) (CallFunction|GetTotalMagAtk (LocalVariables|GetAttackerDamageCalsComponent)) (CallFunction|GetTotalPhyAtk (LocalVariables|GetAttackerDamageCalsComponent))) (|CalcDef (LocalVariables|GetisMagic)) (select (LocalVariables|GetIsCritical) (LocalVariables|GetSumCriticalDamageRatio) 1.0)))
      (Development|PrintText (Utilities|Text|ToText(Float) DamageAmount "HalfToEven") true true "(R=0.000000,G=0.660000,B=1.000000,A=1.000000)" 2.0 "Damage")
      (return))
    (:Fail
      (return))))

(fn GetTotalPhyAtk
  (return (Variables|Default|GetPhysicDamage)))

(fn GetTotalMagAtk
  (return (Variables|Default|GetMagicDamage)))

(fn ApplyBaseParams
  (params (BaseParams :type Character%20Param%20Structure))
  (bind (_physicdamage _magicdamage _hp _def _magicdef _attackspeedrate _movementspeedrate _reducecooldownratio _criticalratio _healhp _piercedef _piercemagicdef _debuffresistanceratio) (Utilities|Struct|BreakCharacterParam BaseParams))
  (Variables|Default|SetPhysicDamage _physicdamage)
  (Variables|Default|SetMagicDamage _magicdamage)
  (Variables|Default|SetDef _def)
  (Variables|Default|SetMagicDef _magicdef)
  (Variables|Default|SetPierceDef _piercedef)
  (Variables|Default|SetPierceMagicDef _piercemagicdef)
  (Variables|Default|SetCriticalRatio _debuffresistanceratio))

(fn CalcCriticalRatio
  (Variables|Default|SetCriticalRatio (Variables|Default|GetCriticalRatio))
  (LocalVariables|SetSumCritDamageRatio 2.0)
  (return (LocalVariables|GetSumCritRatio) (LocalVariables|GetSumCritDamageRatio)))

(fn ParsingDamageCalcInfo
  (params (DamageCalcComponent :type Damage%20Cals%20Component%20Object%20Reference))
  (Utilities|FlowControl|Sequence
    (:then_0
      (Variables|Default|SetPhysicDamage (Variables|DamageCalsComponent_C|GetPhysicDamage DamageCalcComponent)))
    (:then_1
      (Variables|Default|SetMagicDamage (Variables|DamageCalsComponent_C|GetMagicDamage DamageCalcComponent)))
    (:then_2
      (Variables|Default|SetPierceDef (Variables|DamageCalsComponent_C|GetPierceDef DamageCalcComponent)))
    (:then_3
      (Variables|Default|SetPierceMagicDef (Variables|DamageCalsComponent_C|GetPierceMagicDef DamageCalcComponent)))
    (:then_4
      (Variables|Default|SetCriticalRatio (Variables|DamageCalsComponent_C|GetCriticalRatio DamageCalcComponent)))))